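; BP_Gigagull is an actor, by name a giant gull, that makes repeated fly-by passes from its placed position.
; BeginPlay stores the start location and starts a looping timer whose interval is randomized once.
; Each tick of that timer picks a random X offset and restarts a Timeline.
; The Timeline lerps the actor from the stored start toward a point far along +Y and higher up, without sweeping.
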(event `self.ReceiveBeginPlay`
  (set `self.New Location` (`self.K2_GetActorLocation`))
  (`KismetSystemLibrary.K2_SetTimerDelegate` (delegate `CustomEvent_0`) (`KismetMathLibrary.RandomFloatInRange` 10.0 60.0) true))

(event `CustomEvent_0`
  (set `self.Xspawn` (`KismetMathLibrary.RandomFloatInRange` -4000.0 4000.0))
  (bind (_direction _newtrack_0) (`Timeline|Timeline_0` :!via `PlayFromStart`)
    (:`Update`
      (`SceneComponent.K2_SetWorldLocation` (`self.RootComponent`) (`KismetMathLibrary.VLerp` (`self.New Location`) (+ (`self.New Location`) (`KismetMathLibrary.MakeVector` (`self.Xspawn`) 15000.0 1500.0)) _newtrack_0) false false))))

(fn `UserConstructionScript`)