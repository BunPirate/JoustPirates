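; Player controller for a boat game that relays player input to its possessed boat character.
; Forward and turn axes pass straight through to the character, and boost fires when the action is released.
; InitController stores the game mode, character and camera references, possesses and initializes the boat with player number and color, then views through the supplied camera in Game and UI input mode.
; Possession prints the pawn's name on screen for debugging.
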(event `InputAction|Boost`
  (params (Key :type "Key Structure"))
  (:`Released`
    (`/Game/Blueprints/Character/P_BoatCharacter.Boost` (`self.Character Ref`))))

(event `InputAxis|MoveShipForward`
  (params (AxisValue :type "Float (single-precision)"))
  (`/Game/Blueprints/Character/P_BoatCharacter.ShipForward` (`self.Character Ref`) AxisValue))

(event `InputAxis|TurnShipRight`
  (params (AxisValue :type "Float (single-precision)"))
  (`/Game/Blueprints/Character/P_BoatCharacter.TurnShipRight` (`self.Character Ref`) AxisValue))

(event `InitController`
  (params (GM :type "/Game/Blueprints/GameMode/GM_main Object Reference") (CharacterRef :type "/Game/Blueprints/Character/P_BoatCharacter Object Reference") (Camera :type "/Game/Blueprints/Camera/BP_Camera Object Reference") (PlayerNumber :type Integer) (InColor :type "LinearColor Structure"))
  (set `self.GMRef` GM)
  (bind _output_get (set `self.Character Ref` CharacterRef))
  (set `self.CameraRef` Camera)
  (`self.Possess` _output_get)
  (`/Game/Blueprints/Character/P_BoatCharacter.InitBoatCharacter` _output_get self (`self.GMRef`) PlayerNumber InColor)
  (`self.SetViewTargetWithBlend` (`self.CameraRef`))
  (`WidgetBlueprintLibrary.SetInputMode_GameAndUIEx` self null))

(event `self.ReceivePossess`
  (params (PossessedPawn :type "Pawn Object Reference"))
  (`KismetSystemLibrary.PrintString` (`KismetSystemLibrary.GetDisplayName` PossessedPawn) true true (struct :`R` 1.0 :`G` 0.826668 :`A` 1.0) 10.0))

(fn `UserConstructionScript`)