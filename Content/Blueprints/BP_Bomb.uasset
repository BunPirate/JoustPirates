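; BP_Bomb is a colour-tinted bomb that damages boats on contact.
; InitBomb tints the cylinder via a dynamic material and starts a timer that arms it a second later.
; Boats, found via GetBoatMessage, get only a mutual nudge before arming.
; Once armed, the first hit damages and shoves the boat, swaps the cylinder for a tinted destructible shattered by radius damage, spawns a Niagara explosion, then destroys the actor after a delay.
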(event `InitBomb`
  (params (Value :type "LinearColor Structure"))
  (set `self.Coloiur` Value)
  (`KismetSystemLibrary.K2_SetTimerDelegate` (delegate `NowExplosive`) 1.0)
  (bind _returnvalue (`PrimitiveComponent.CreateDynamicMaterialInstance` (`self.Cylinder`) 0 "/Game/Materials/Pirate_Ship/M_ShipRed_Inst.M_ShipRed_Inst" "None"))
  (`MaterialInstanceDynamic.SetVectorParameterValue` _returnvalue "Colour" Value))

(event `NowExplosive`
  (set `self.Explosive?` true))

(event `self.ReceiveHit`
  (params (MyComp :type "PrimitiveComponent Object Reference") (Other :type "Actor Object Reference") (OtherComp :type "PrimitiveComponent Object Reference") (bSelfMoved :type Boolean) (HitLocation :type "Vector Structure") (HitNormal :type "Vector Structure") (NormalImpulse :type "Vector Structure") (Hit :type "HitResult Structure (by ref)"))
  (bind _cylinder (`self.Cylinder`))
  (bind _cylinder_2 (`self.Cylinder`))
  (bind _boatref (message `/Game/Blueprints/Character/BPI_Boat.GetBoat` Other))
  (`/Engine/EditorBlueprintResources/StandardMacros.IsValid` _boatref
    (:`Is Valid`
      (if (`self.Explosive?`)
        (`/Engine/EditorBlueprintResources/StandardMacros.DoOnce` false
          (:`Completed`
            (bind _boat (`/Game/Blueprints/Character/P_BoatCharacter.Boat` _boatref))
            (`PrimitiveComponent.AddImpulseAtLocation` _boat (1000.0 1000.0 1000.0) HitLocation "None")
            (`/Game/Blueprints/Character/P_BoatCharacter.ApplyDamage` _boatref 30)
            (`SceneComponent.SetHiddenInGame` _cylinder_2 true false)
            (`PrimitiveComponent.SetSimulatePhysics` _cylinder_2 false)
            (`PrimitiveComponent.SetCollisionEnabled` _cylinder_2 "NoCollision")
            (bind _returnvalue (`AddComponent|NODE_AddDestructibleComponent-0` :`RelativeTransform` (`KismetMathLibrary.MakeTransform` (0.0 0.0 0.0) (`SceneComponent.K2_GetComponentRotation` _cylinder))))
            (bind _returnvalue_2 (`PrimitiveComponent.CreateDynamicMaterialInstance` _returnvalue 0 "/Game/Materials/Pirate_Ship/M_ShipRed_Inst.M_ShipRed_Inst" "None"))
            (`MaterialInstanceDynamic.SetVectorParameterValue` _returnvalue_2 "Colour" (`self.Coloiur`))
            (`NiagaraFunctionLibrary.SpawnSystemAtLocation` "/Game/Effects/NS_Explosion.NS_Explosion" (`SceneComponent.K2_GetComponentLocation` (`self.Cylinder`)) (struct) (10.0 10.0 10.0))
            (`DestructibleComponent.ApplyRadiusDamage` _returnvalue 100.0 (`SceneComponent.K2_GetComponentLocation` _cylinder) 1000.0 10000.0 false)
            (`KismetSystemLibrary.K2_SetTimerDelegate` (delegate `Destroy`) 5.0)))
        (else
          (`PrimitiveComponent.AddImpulse` _boat (200.0 200.0 200.0) "None" false)
          (`PrimitiveComponent.AddImpulse` (`self.Cylinder`) (200.0 200.0 200.0) "None" false))))))

(event `Destroy`
  (`self.K2_DestroyActor`))

(fn `UserConstructionScript`)