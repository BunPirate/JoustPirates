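; Main menu pawn that displays a slowly spinning character mesh as a preview.
; BeginPlay hides the mesh and starts a looping timer that nudges its yaw, and ShowCharacterPreview makes it visible with its children.
; GetMenuPawn returns the pawn itself.
; Next and previous mesh events are empty stubs, and a SetSkeletalMesh call is left unconnected, so character switching is not implemented.
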(event `self.ReceiveBeginPlay`
  (`KismetSystemLibrary.K2_SetTimerDelegate` (delegate `Rotate`) 0.01 true)
  (`SceneComponent.SetVisibility` (`self.CharacterMesh`) false true))

(event `Rotate`
  (`SceneComponent.K2_AddLocalRotation` (`self.CharacterMesh`) (struct :`Yaw` 0.25) false false))

(event `ShowCharacterPreview`
  (`SceneComponent.SetVisibility` (`self.CharacterMesh`) true true))

(event `NextCharacterMesh`)

(event `PreviousCharacterMesh`)

(fn `GetMenuPawn`
  (returns (MenuPawn :type "/Game/Blueprints/Character/BP_MainMenuPawn Object Reference"))
  (return self))

(fn `UserConstructionScript`)