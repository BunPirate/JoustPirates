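; BP_RandomRock is an environment actor that scatters randomized rock meshes beneath its Box volume at construction.
; The construction script clears Regenerate, then traces from random box points toward separately randomized points far below.
; Each trace's hit location, converted to actor space, places a static mesh component with random rotation and per-axis scale.
; Each mesh gets a dynamic M_Rock_Inst material with random Tint; hit success is never checked.
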(fn `UserConstructionScript`
  (bind _returnvalue (`KismetMathLibrary.RandomFloatInRange` 5.0 15.0))
  (bind _box (`self.Box`))
  (bind _returnvalue_2 (`KismetMathLibrary.RandomPointInBoundingBox` (`SceneComponent.K2_GetComponentLocation` _box) (`BoxComponent.GetScaledBoxExtent` _box)))
  (set `self.Regenerate` false)
  (for _ (range (+ (`KismetMathLibrary.RandomIntegerInRange` 10 20) 1))
    (bind _outhit (`KismetSystemLibrary.LineTraceSingle` _returnvalue_2 (- _returnvalue_2 (0.0 0.0 10000.0)) "TraceTypeQuery1"))
    (bind _returnvalue_3 (`AddComponent|NODE_AddStaticMeshComponent-0` :`RelativeTransform` (`KismetMathLibrary.MakeRelativeTransform` (`KismetMathLibrary.MakeTransform` (`.Location` (`GameplayStatics.BreakHitResult` _outhit)) (`KismetMathLibrary.RandomRotator` true) (`KismetMathLibrary.MakeVector` _returnvalue _returnvalue _returnvalue)) (`self.GetTransform` self))))
    (bind _returnvalue_4 (`KismetMaterialLibrary.CreateDynamicMaterialInstance` "/Game/Meshes/ROCKS/M_Rock_Inst.M_Rock_Inst"))
    (`MaterialInstanceDynamic.SetScalarParameterValue` _returnvalue_4 "Tint" (`KismetMathLibrary.RandomFloatInRange` -1.0 2.0))
    (`PrimitiveComponent.SetMaterial` _returnvalue_3 0 _returnvalue_4)))