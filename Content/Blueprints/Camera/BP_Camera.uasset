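; A shared camera actor that follows the group of boat characters passed to it through Initcamera.
; Each Tick it averages the locations of all stored characters and moves itself to that midpoint plus a fixed offset behind and above.
; The move is an instant, unswept location set with no smoothing, and rotation is never changed.
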(event `Initcamera`
  (params (BoatCharacters :type "Array of /Game/Blueprints/Character/P_BoatCharacter Object Reference"))
  (set `self.Boat Characters` BoatCharacters))

(event `self.ReceiveTick`
  (params (DeltaSeconds :type "Float (single-precision)"))
  (bind _boat_characters (`self.Boat Characters`))
  (set `self.TotalLocation` (0.0 0.0 0.0))
  (for _array_element _boat_characters
    (set `self.TotalLocation` (+ (`self.TotalLocation`) (`self.K2_GetActorLocation` _array_element))))
  (`self.K2_SetActorLocation` (+ (/ (`self.TotalLocation`) (`KismetArrayLibrary.Array_Length` _boat_characters)) (-1760.0 0.0 3020.0))))

(fn `UserConstructionScript`)