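; BP_OverlapBorderVolume is a border volume that knocks back boats that stay inside it.
; When an actor implementing BPI_Boat enters the Box, it stores the boat reference and starts a two-second one-shot timer, which is cleared on exit.
; When the timer fires, it applies a Force-scaled impulse to the boat toward a fixed world point above the origin.
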(event `self.Box.OnComponentBeginOverlap`
  (params (OverlappedComponent :type "PrimitiveComponent Object Reference") (OtherActor :type "Actor Object Reference") (OtherComp :type "PrimitiveComponent Object Reference") (OtherBodyIndex :type Integer) (bFromSweep :type Boolean) (SweepResult :type "HitResult Structure (by ref)"))
  (if (`KismetSystemLibrary.DoesImplementInterface` OtherActor "/Game/Blueprints/Character/BPI_Boat.BPI_Boat_C")
    (bind _boatref (message `/Game/Blueprints/Character/BPI_Boat.GetBoat` OtherActor))
    (set `self.Boat Ref` _boatref)
    (set `self.IsOverlapping?` true)
    (bind _returnvalue (`KismetSystemLibrary.K2_SetTimerDelegate` (delegate `BoatKnockback`) 2.0))
    (set `self.KnockbackHandle` _returnvalue)
    (`KismetSystemLibrary.PrintString` "Overlapped")))

(event `BoatKnockback`
  (bind _boat_ref (`self.Boat Ref`))
  (`PrimitiveComponent.AddImpulse` (`/Game/Blueprints/Character/P_BoatCharacter.Boat` _boat_ref) (* (`KismetMathLibrary.GetDirectionUnitVector` (`self.K2_GetActorLocation` _boat_ref) (0.0 0.0 1000.0)) (`self.Force`)) "None" false)
  (`KismetSystemLibrary.PrintString` "Impulse added"))

(event `self.Box.OnComponentEndOverlap`
  (params (OverlappedComponent :type "PrimitiveComponent Object Reference") (OtherActor :type "Actor Object Reference") (OtherComp :type "PrimitiveComponent Object Reference") (OtherBodyIndex :type Integer))
  (if (`KismetSystemLibrary.DoesImplementInterface` OtherActor "/Game/Blueprints/Character/BPI_Boat.BPI_Boat_C")
    (message `/Game/Blueprints/Character/BPI_Boat.GetBoat` OtherActor)
    (set `self.IsOverlapping?` false)
    (`KismetSystemLibrary.K2_ClearAndInvalidateTimerHandle` (`self.KnockbackHandle`))))

(fn `UserConstructionScript`)