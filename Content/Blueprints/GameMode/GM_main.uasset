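; Game mode that sets up a local multiplayer boat match with a shared camera and timed pickups.
; On BeginPlay it gathers spawn points, spawns the camera, recreates local players from the game instance's count, and spawns a boat for each.
; An init chain hands each controller its boat, camera, number and color, then passes all boats to the camera.
; A looping timer spawns pickups at random points inside the pickup zone.
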(event `self.ReceiveBeginPlay`
  (`self.SetupSpawnPoint`)
  (`self.SetupCamera`)
  (`self.SetupController`)
  (`self.SetupCharacter`)
  (`self.InitChain`)
  (`self.StartPowerUpSpawn`)
  (bind _returnvalue (`GameplayStatics.GetActorOfClass` "/Game/Blueprints/GameMode/BP_PickupSpawnZone.BP_PickupSpawnZone_C"))
  (set `self.SpawnZone` _returnvalue))

(event `StartPowerUpSpawn`
  (bind _returnvalue (`KismetSystemLibrary.K2_SetTimerDelegate` (delegate `SpawnPowerup`) 10.0 true))
  (set `self.SpawnPickupHandle` _returnvalue))

(event `SpawnPowerup`
  (bind _spawnzone (`self.SpawnZone`))
  (`|SpawnActorFromClass` "/Game/Blueprints/GameMode/BP_Pickup.BP_Pickup_C" (`KismetMathLibrary.MakeTransform` (`KismetMathLibrary.RandomPointInBoundingBox` (`SceneComponent.K2_GetComponentLocation` (`Actor.RootComponent` _spawnzone)) (`/Game/Blueprints/GameMode/BP_PickupSpawnZone.In Box Extent` _spawnzone))) "Undefined" "OverrideRootScale" null null))

(fn `InitChain`
  ;[1 1 1] InitController
  (for (_array_element _array_index) (`self.ControllerRefs`)
    (`KismetSystemLibrary.PrintString` (`KismetStringLibrary.Concat_StrStr` "Controller:" (`KismetSystemLibrary.GetDisplayName` _array_element)))
    (`/Game/Blueprints/Controller/PC_CustomControlelr.InitController` _array_element self (`|GetArrayItem` (`self.CharacterRef`) _array_index) (`self.CameraRef`) (+ _array_index 1) (select `int` _array_index :`0` (struct :`R` 1.0 :`A` 1.0) :`1` (struct :`G` 0.002072 :`B` 1.0 :`A` 1.0) :`2` (struct :`R` 0.041786 :`G` 1.0 :`A` 1.0) :`3` (struct :`R` 1.0 :`B` 0.633862 :`A` 1.0) :`4` (struct :`G` 1.0 :`B` 0.964648 :`A` 1.0) :!type "LinearColor Structure")))
  (`/Game/Blueprints/Camera/BP_Camera.Initcamera` (`self.CameraRef`) (`self.CharacterRef`)))

(fn `SetupCamera`
  (bind _returnvalue (`|SpawnActorFromClass` "/Game/Blueprints/Camera/BP_Camera.BP_Camera_C" (`KismetMathLibrary.MakeTransform` (-1760.0 0.0 3020.0)) "Undefined" "OverrideRootScale" null null))
  (set `self.CameraRef` _returnvalue))

(fn `SetupCharacter`
  (for (_ _array_index) (`self.ControllerRefs`)
    (bind _output (`|GetArrayItem` (`self.SpawnPoint`) _array_index))
    (bind _returnvalue (`|SpawnActorFromClass` "/Game/Blueprints/Character/P_BoatCharacter.P_BoatCharacter_C" (`KismetMathLibrary.MakeTransform` (`/Game/Blueprints/Character/BP_SpawnPoint.SpawnLocation` _output) (`/Game/Blueprints/Character/BP_SpawnPoint.SpawnRotation` _output)) "Undefined" "OverrideRootScale" null null))
    (`KismetArrayLibrary.Array_Add` (`self.CharacterRef`) _returnvalue)))

(fn `SetupController`
  (`GameplayStatics.RemovePlayer` (`GameplayStatics.GetPlayerController` 0))
  (for _ (range (`/Game/Blueprints/GameMode/GI_Main.NumberOfPlayers` (cast `/Game/Blueprints/GameMode/GI_Main` (`GameplayStatics.GetGameInstance`) :!pure true)))
    (bind _returnvalue (`GameplayStatics.CreatePlayer` -1))
    (`KismetArrayLibrary.Array_Add` (`self.ControllerRefs`) (cast `/Game/Blueprints/Controller/PC_CustomControlelr` _returnvalue :!pure true))))

(fn `SetupSpawnPoint`
  (bind _outactors (`GameplayStatics.GetAllActorsOfClass` "/Game/Blueprints/Character/BP_SpawnPoint.BP_SpawnPoint_C"))
  (bind _output_get (set `self.SpawnPoint` _outactors))
  (for _array_element _output_get
    (`/Game/Blueprints/Character/BP_SpawnPoint.InitSpawnPoint` _array_element)))

(fn `UserConstructionScript`)